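; BP_BasicAIDirector is an AI director that switches every queried planner to a shared goal, either attack or patrol.
; AllAttack and AllPatrol pass their goal to SetAllGoal, which gets the planners from QueryAllPlanners and calls SetGoal on each.
; After the loop, it prints the new goal's name as a magenta director order for debugging.
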(fn ConstructionScript)

(fn SetAllGoal
  (params (NewGoal :type SP%20Goal%20Object%20Reference))
  (bind _returnvalue (Class|SPAIDirector|QueryAllPlanners))
  (for _array_element _returnvalue
    (Class|SPPlannerComponent|SetGoal _array_element NewGoal))
  (Development|PrintString (Utilities|String|Append "AIDirector Order: " (Utilities|GetObjectName NewGoal)) true true "(R=1.000000,G=0.000000,B=1.000000,A=1.000000)"))

(fn AllAttack
  (CallFunction|SetAllGoal (Variables|Default|GetAttackGoal)))

(fn AllPatrol
  (CallFunction|SetAllGoal (Variables|Default|GetPatrolGoal)))