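; Demo player controller that switches AI planner goals from hotkeys and leads a formation with the player's pawn.
; The O, P, L and K keys set the attack, patrol, formation or idle goal on selected planners, or on all if none are selected, through a singleton instance.
; BeginPlay makes the controlled pawn the lead actor of an SP_FormationSet, and EndPlay resets that set.
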(event EventBeginPlay
  (bind _assp_formation_set (Utilities|Casting|CastToSP_FormationSet (Class|SPBlueprintHelper|GetObject "/Game/Blueprints/AI/Formations/FormationSet.FormationSet")))
  (Class|SPFormationSet|SetLeadActor _assp_formation_set (Pawn|GetControlledPawn)))

(event EventEndPlay
  (params (EndPlayReason :type EEndPlayReason%20Enum :default "Destroyed"))
  (bind _assp_formation_set (Utilities|Casting|CastToSP_FormationSet (Class|SPBlueprintHelper|GetObject "/Game/Blueprints/AI/Formations/FormationSet.FormationSet")))
  (Class|SPFormationSet|Reset _assp_formation_set))

(event Input|KeyboardEvents|K
  (params (Key :type Key%20Structure))
  (:Pressed
    (Class|SPDirector|SetAllSelectedPlannerGoal (Class|SPDirector|GetInstance) "/Game/Blueprints/AI/Goals/IdleGoal.IdleGoal" true)))

(event Input|KeyboardEvents|O
  (params (Key :type Key%20Structure))
  (:Pressed
    (Class|SPDirector|SetAllSelectedPlannerGoal (Class|SPDirector|GetInstance) "/Game/Blueprints/AI/Goals/AttackGoal.AttackGoal" true)))

(event Input|KeyboardEvents|P
  (params (Key :type Key%20Structure))
  (:Pressed
    (Class|SPDirector|SetAllSelectedPlannerGoal (Class|SPDirector|GetInstance) "/Game/Blueprints/AI/Goals/PatrolGoal.PatrolGoal" true)))

(event Input|KeyboardEvents|L
  (params (Key :type Key%20Structure))
  (:Pressed
    (Class|SPDirector|SetAllSelectedPlannerGoal (Class|SPDirector|GetInstance) "/Game/Blueprints/AI/Goals/FormationGoal.FormationGoal" true)))

(fn ConstructionScript)